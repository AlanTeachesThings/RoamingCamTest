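; Minimap scanner actor that, as written, only visualizes a grid of sample points across its own bounds.
; ScanWithinBounds takes the actor's XY bounds extent and steps from the minimum corner in nested loops at the given spacing.
; Each point gets a short-lived red debug sphere at a fixed world height, with no tracing or map capture.
; BeginPlay and the construction script are empty, so nothing here calls the scan.
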(event EventBeginPlay)

(fn ConstructionScript)

(fn ScanWithinBounds
  (params (Spacing :type Float%20%28double-precision%29))
  (bind _boxextent (Collision|GetActorBounds false false))
  (LocalVariables|SetBoundsXY (Math|Vector2D|MakeVector2D (.x _boxextent) (.y _boxextent)))
  (for _index (range 0 (Math|Float|Ceil (/ (* (.x (LocalVariables|GetBoundsXY)) 2.0) Spacing)))
    (for _index_2 (range 0 (Math|Float|Ceil (/ (* (.y (LocalVariables|GetBoundsXY)) 2.0) Spacing)))
      (Rendering|Debug|DrawDebugSphere (Math|Vector|MakeVector (.x (+ (- (Transformation|GetActorLocation) (Math|Vector|MakeVector (.x (LocalVariables|GetBoundsXY)) (.y (LocalVariables|GetBoundsXY)) 0.0)) (Math|Vector|MakeVector (* _index Spacing) (* _index_2 Spacing) 0.0))) (.y (+ (- (Transformation|GetActorLocation) (Math|Vector|MakeVector (.x (LocalVariables|GetBoundsXY)) (.y (LocalVariables|GetBoundsXY)) 0.0)) (Math|Vector|MakeVector (* _index Spacing) (* _index_2 Spacing) 0.0))) 3e+02) 1e+01 12 "(R=1.000000,G=0.000000,B=0.000000,A=1.000000)" 1.0 3.0))))